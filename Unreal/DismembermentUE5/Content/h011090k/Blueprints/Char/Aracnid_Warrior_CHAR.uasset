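; Arachnid warrior character Blueprint with per-limb dismemberment for legs, mandibles and lower jaw, each a separate skeletal mesh component.
; Point damage maps the hit bone to a component by name and bone hierarchy, adding the child segment for upper legs.
; DamageLimb lowers the first listed limb with remaining health, then immediately replaces its mesh with a physics-simulated BP_LostBits copy, even if health remains.
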(event Custom|Multi_SpawnLimb
  (params (SKM_ToSpawn :type Skeletal%20Mesh%20Object%20Reference) (MeshToHide :type Skeletal%20Mesh%20Component%20Object%20Reference))
  (Components|DestroyComponent MeshToHide)
  (bind _returnvalue (Game|SpawnActorfromClass "/Game/h011090k/Blueprints/Char/BP_LostBits.BP_LostBits_C" (Transformation|GetWorldTransform (Variables|Character|GetMesh)) "AlwaysSpawn" "MultiplyWithRoot" 0 0))
  (Components|SkinnedMesh|SetSkinnedAssetandUpdate (Variables|/Game/h011090k/Blueprints/Char/BP_LostBits.BP_LostBits_C|GetSkeletalMesh _returnvalue) SKM_ToSpawn false)
  (Collision|SetCollisionEnabled (Variables|/Game/h011090k/Blueprints/Char/BP_LostBits.BP_LostBits_C|GetSkeletalMesh _returnvalue) "PhysicsOnly")
  (Physics|SetSimulatePhysics (Variables|/Game/h011090k/Blueprints/Char/BP_LostBits.BP_LostBits_C|GetSkeletalMesh _returnvalue) true)
  (Physics|AddImpulse (Variables|/Game/h011090k/Blueprints/Char/BP_LostBits.BP_LostBits_C|GetSkeletalMesh _returnvalue) (Math|Vector|MakeVector 0.0 0.0 0.0) "None" true)
  (Class|PrimitiveComponent|SetMassOverrideinKg (Variables|/Game/h011090k/Blueprints/Char/BP_LostBits.BP_LostBits_C|GetSkeletalMesh _returnvalue) "None" 1e+06 true))

(event Game|Damage|EventPointDamage
  (params (Damage :type Float%20%28single-precision%29) (DamageType :type Damage%20Type%20Object%20Reference) (HitLocation :type Vector :default "0, 0, 0") (HitNormal :type Vector :default "0, 0, 0") (HitComponent :type Primitive%20Component%20Object%20Reference) (BoneName :type Name :default "None") (ShotFromDirection :type Vector :default "0, 0, 0") (InstigatedBy :type Controller%20Object%20Reference) (DamageCauser :type Actor%20Object%20Reference) (HitInfo :type Hit%20Result%20Structure%20%28by%20ref%29))
  (Variables|Default|SetDamage Damage)
  (Variables|Default|SetBone%20Name BoneName)
  (bind (_itemtodismember _dismember_) (CallFunction|GetDamagedLimb))
  (if _dismember_
    (bind _outputlimbs (CallFunction|IsSubLimb _itemtodismember))
    (bind _limbdestroyed_ (CallFunction|DamageLimb _outputlimbs))
    (if _limbdestroyed_
      _)))

(fn ConstructionScript
  (Variables|Default|SetAllDismemberableComponents (Utilities|Array|MakeArray 0 (Variables|Default|GetDEF_Mandible_1_L) (Variables|Default|GetDEF_Leg_10_R) (Variables|Default|GetDEF_Leg_12_L) (Variables|Default|GetDEF_Mandible_1_R) (Variables|Default|GetDEF_Leg_12_R) (Variables|Default|GetDEF_Leg_10_L) (Variables|Default|GetDEF_Leg_02_L) (Variables|Default|GetDEF_Leg_00_L) (Variables|Default|GetDEF_JawLower) (Variables|Default|GetDEF_Leg_00_R) (Variables|Default|GetDEF_Leg_02_R)))
  (Utilities|FlowControl|Sequence
    (:then_0
      ;[1 1 1] Front Legs
      ;;[1 1 1] Right
      (Utilities|Map|Add (Variables|Default|GetLimbHealth) (Variables|Default|GetDEF_Leg_02_R) 2e+01)
      (Utilities|Map|Add (Variables|Default|GetLimbHealth) (Variables|Default|GetDEF_Leg_00_R) 2e+01)
      ;;[1 1 1] Left
      (Utilities|Map|Add (Variables|Default|GetLimbHealth) (Variables|Default|GetDEF_Leg_00_L) 2e+01)
      (Utilities|Map|Add (Variables|Default|GetLimbHealth) (Variables|Default|GetDEF_Leg_02_L) 2e+01))
    (:then_1
      ;[1 1 1] Rear Legs
      ;;[1 1 1] Right
      (Utilities|Map|Add (Variables|Default|GetLimbHealth) (Variables|Default|GetDEF_Leg_12_R) 2e+01)
      (Utilities|Map|Add (Variables|Default|GetLimbHealth) (Variables|Default|GetDEF_Leg_10_R) 2e+01)
      ;;[1 1 1] Left
      (Utilities|Map|Add (Variables|Default|GetLimbHealth) (Variables|Default|GetDEF_Leg_12_R) 2e+01)
      (Utilities|Map|Add (Variables|Default|GetLimbHealth) (Variables|Default|GetDEF_Leg_10_L) 2e+01))
    (:then_2
      ;[1 1 1] Stabby's
      ;;[1 1 1] Right
      (Utilities|Map|Add (Variables|Default|GetLimbHealth) (Variables|Default|GetDEF_Mandible_1_R) 2e+01)
      ;;[1 1 1] Left
      (Utilities|Map|Add (Variables|Default|GetLimbHealth) (Variables|Default|GetDEF_Mandible_1_L) 2e+01))
    (:then_3
      ;[1 1 1] Misc
      ;;[1 1 1] Jaw
      (Utilities|Map|Add (Variables|Default|GetLimbHealth) (Variables|Default|GetDEF_JawLower) 2e+01))))

(fn GetDamagedLimb
  (bind _bone_name (Variables|Default|GetBone%20Name))
  (for _array_element (Variables|Default|GetAllDismemberableComponents)
    ;[1 1 1] Itteratively Check through all existing limbs
    (Utilities|IsValid _array_element
      (:Is%20Valid
        (if (or (Class|SkinnedMeshComponent|BoneIsChildOf _array_element _bone_name (Utilities|String|StringToName (Utilities|GetObjectName _array_element))) (== _bone_name (Utilities|String|StringToName (Utilities|GetObjectName _array_element))))
          (return _array_element true)))))
  ;[1 1 1] If it is not any existing dismemberable bones  - Stop
  (return 0 false))

(fn DamageLimb
  (params (Limb :type Array%20of%20Skeletal%20Mesh%20Component%20Object%20References))
  (for _array_element Limb
    (if (and (> (.Value (Utilities|Map|Find (Variables|Default|GetLimbHealth) _array_element)) 0.0) (.ReturnValue (Utilities|Map|Find (Variables|Default|GetLimbHealth) _array_element)))
      (Utilities|Map|Add (Variables|Default|GetLimbHealth) _array_element (Math|Float|SelectFloat (- (.Value (Utilities|Map|Find (Variables|Default|GetLimbHealth) _array_element)) (Variables|Default|GetDamage)) 0.0 (> (- (.Value (Utilities|Map|Find (Variables|Default|GetLimbHealth) _array_element)) (Variables|Default|GetDamage)) 0.0)))
      (CallFunction|MultiSpawnLimb (Components|SkeletalMesh|GetSkeletalMeshAsset _array_element) _array_element)
      (return (<= (.Value (Utilities|Map|Find (Variables|Default|GetLimbHealth) _array_element)) 0.0)))))

(fn GetDamagedLimb0
  (bind _bone_name (Variables|Default|GetBone%20Name))
  (bind _def_leg_12_r (Variables|Default|GetDEF_Leg_12_R))
  (bind _bone_name_2 (Variables|Default|GetBone%20Name))
  (bind _def_leg_10_r (Variables|Default|GetDEF_Leg_10_R))
  ;[1 0.6561 0.8575] Rear
  ;;[1 1 1] Right
  ;;;[0.8202 0.97 1] Rear Leg (End)
  (Utilities|IsValid _def_leg_12_r
    (:Is%20Valid
      (if (or (Class|SkinnedMeshComponent|BoneIsChildOf _def_leg_12_r _bone_name_2 "DEF_Leg_11_R") (== _bone_name_2 "DEF_Leg_11_R"))
        (return true _def_leg_12_r)
        (else
          _)))
    (:Is%20Not%20Valid
      _))
  ;;;[0.8639 1 0.8079] Rear Leg (Main)
  (Utilities|IsValid _def_leg_10_r
    (:Is%20Valid
      (if (or (Class|SkinnedMeshComponent|BoneIsChildOf _def_leg_10_r _bone_name "DEF_Leg_10_R") (== _bone_name "DEF_Leg_10_R"))
        (return true _def_leg_10_r)))))

(fn IsSubLimb
  (params (InputLimb :type Skeletal%20Mesh%20Component%20Object%20Reference))
  (bind _returnvalue (Utilities|String|ToString(Object) InputLimb))
  (bind _returnvalue_2 (Utilities|String|Contains _returnvalue "Leg" true))
  (LocalVariables|SetInput%20Limb InputLimb)
  (LocalVariables|SetNameOfInputLimb _returnvalue)
  (Development|PrintString (Utilities|String|ToString(Boolean) _returnvalue_2))
  (if _returnvalue_2
    (if (Utilities|String|Contains (LocalVariables|GetNameOfInputLimb) "0_" true)
      (Development|PrintString "IS PART OF CHAIN")
      (bind _asskeletal_mesh_component (Utilities|Casting|CastToSkeletalMeshComponent (Components|GetChildComponent (LocalVariables|GetInput%20Limb) 0)))
      (Development|PrintString (Utilities|String|ToString(Object) (LocalVariables|GetInput%20Limb)))
      (Development|PrintString (Utilities|String|ToString(Object) _asskeletal_mesh_component))
      (return true (Utilities|Array|MakeArray (LocalVariables|GetInput%20Limb) _asskeletal_mesh_component))
      (else
        _)))
  (return false (Utilities|Array|MakeArray (LocalVariables|GetInput%20Limb))))